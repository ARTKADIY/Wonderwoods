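; BP_Mshyvets is a mob actor that patrols back and forth along its local X axis.
; Tick accumulates time, moving the actor forward at a fixed speed for SecondsBeforeReturning, then backward for the same period, before resetting the timer.
; A Stop event pauses movement for two seconds through a flag, while the timer keeps accumulating.
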(event EventTick
  (params (DeltaSeconds :type Float%20%28single-precision%29))
  (bind _returnvalue (* 100 DeltaSeconds))
  (bind _secondsbeforereturning (Variables|Default|GetSecondsBeforeReturning))
  (bind _output_get (Variables|Default|Setsec (+ DeltaSeconds (Variables|Default|Getsec))))
  (if (not (Variables|Default|GetIsStopping))
    (if (<= _output_get (Math|Conversions|ToFloat(Integer) _secondsbeforereturning))
      (Transformation|AddActorLocalOffset (Math|Vector|MakeVector _returnvalue 0.0 0.0) false false)
      (elif (<= (Variables|Default|Getsec) (Math|Conversions|ToFloat(Integer) (* _secondsbeforereturning 2)))
        (Transformation|AddActorLocalOffset (Math|Vector|MakeVector (* -1 _returnvalue) 0.0 0.0) false false)
        (else
          (Variables|Default|Setsec 0.0))))))

(event EventStop
  (Variables|Default|SetIsStopping true)
  (Utilities|FlowControl|Delay 2.0)
  (Variables|Default|SetIsStopping false))

(fn ConstructionScript)