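; BP_Morilka is a side-scroller mob that patrols back and forth and damages an overlapping 2DSideScrollerCharacter.
; Tick moves it along local X, reversing after SecondsBeforeReturning, using an accumulated timer.
; Overlap events flag contact, letting Tick subtract one Health on a two-second cooldown, print it and call the character's DEATH.
; A Stop event pauses movement and damage for two seconds, though both timers keep counting.
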(event EventStop
  (Variables|Default|SetIsStopping true)
  (Utilities|FlowControl|Delay 2.0)
  (Variables|Default|SetIsStopping false))

(event EventTick
  (params (DeltaSeconds :type Float%20%28single-precision%29))
  (bind _returnvalue (* 100 DeltaSeconds))
  (bind _secondsbeforereturning (Variables|Default|GetSecondsBeforeReturning))
  (Variables|Default|SetCoolDown (+ DeltaSeconds (Variables|Default|GetCoolDown)))
  (bind _output_get (Variables|Default|Setsec (+ DeltaSeconds (Variables|Default|Getsec))))
  (if (not (Variables|Default|GetIsStopping))
    (Utilities|FlowControl|Sequence
      (:then_0
        (if (and (>= (Variables|Default|GetCoolDown) 2.0) (Variables|Default|GetGettingDamage))
          (bind _output_get_2 (Variables|/Game/2DSideScrollerBP/Blueprints/2DSideScrollerCharacter.2DSideScrollerCharacter_C|SetHealth (stale Collision|EventActorBeginOverlap _as2dside_scroller_character) (- (Variables|/Game/2DSideScrollerBP/Blueprints/2DSideScrollerCharacter.2DSideScrollerCharacter_C|GetHealth (stale Collision|EventActorBeginOverlap _as2dside_scroller_character)) 1)))
          (Development|PrintString (Utilities|String|ToString(Integer) _output_get_2))
          (Variables|Default|SetCoolDown 0.0)
          (Default|DEATH (stale Collision|EventActorBeginOverlap _as2dside_scroller_character))))
      (:then_1
        (if (<= _output_get (Math|Conversions|ToFloat(Integer) _secondsbeforereturning))
          (Transformation|AddActorLocalOffset (Math|Vector|MakeVector _returnvalue 0.0 0.0) false false)
          (elif (<= (Variables|Default|Getsec) (Math|Conversions|ToFloat(Integer) (* _secondsbeforereturning 2)))
            (Transformation|AddActorLocalOffset (Math|Vector|MakeVector (* -1 _returnvalue) 0.0 0.0) false false)
            (else
              (Variables|Default|Setsec 0.0))))))))

(event Collision|EventActorBeginOverlap
  (params (OtherActor :type Actor%20Object%20Reference))
  (bind _as2dside_scroller_character (Utilities|Casting|CastTo2DSideScrollerCharacter OtherActor))
  (Variables|Default|SetGettingDamage true))

(event Collision|EventActorEndOverlap
  (params (OtherActor :type Actor%20Object%20Reference))
  (Utilities|Casting|CastTo2DSideScrollerCharacter OtherActor)
  (Variables|Default|SetGettingDamage false))

(fn ConstructionScript)