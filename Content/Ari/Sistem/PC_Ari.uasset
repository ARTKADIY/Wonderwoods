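; PC_Ari is a player controller that sets up the level and pause widgets and handles opening the pause menu.
; On BeginPlay it adds a hidden WBP_Pause and a WBP_Level to the viewport.
; Pressing Q pauses the game, reveals the pause widget, switches to UI-only input and shows the mouse cursor.
; It contains no resume logic.
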(event EventBeginPlay
  (bind _returnvalue (UserInterface|CreateWidget "/Game/Ari/WBP/WBP_Pause.WBP_Pause_C"))
  (Widget|SetVisibility _returnvalue "Hidden")
  (UserInterface|Viewport|AddtoViewport _returnvalue 0)
  (bind _returnvalue_2 (UserInterface|CreateWidget "/Game/Ari/WBP/WBP_Level.WBP_Level_C"))
  (UserInterface|Viewport|AddtoViewport _returnvalue_2 0))

(event Input|KeyboardEvents|Q
  (params (Key :type Key%20Structure :default "None"))
  (:Pressed
    (Game|SetGamePaused true)
    (Widget|SetVisibility (stale EventBeginPlay _returnvalue) "Visible")
    (Input|SetInputModeUIOnly self 0 "DoNotLock")
    (Variables|Default|SetbShowMouseCursor true)))

(fn ConstructionScript)